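; Door Blueprint, child of a parent door class, that moves its mesh vertically when a BP_Skill_Char enters or leaves the TriggerOpen volume.
; Overlap start records the character and plays the OpenDoor timeline; overlap end plays CloseDoor only for recorded actors.
; Both timelines add Z offsets every update rather than setting positions.
; Busy flags ignore overlaps mid-move, but DoorBusyOpen is set before the character cast.
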(event OnComponentBeginOverlap(TriggerOpen)
  (params (OverlappedComponent :type Primitive%20Component%20Object%20Reference) (OtherActor :type Actor%20Object%20Reference) (OtherComp :type Primitive%20Component%20Object%20Reference) (OtherBodyIndex :type Integer) (bFromSweep :type Boolean) (SweepResult :type Hit%20Result%20Structure%20%28by%20ref%29))
  (if (not (or (Variables|Default|GetbDoorBusyClose) (Variables|Default|GetbDoorBusyOpen)))
    (if (not (Variables|Default|GetbIsOpenned))
      (Variables|Default|SetbDoorBusyOpen true)
      (Variables|Default|SetbDoorFinishMove false)
      (bind _asbp_skill_char (Utilities|Casting|CastToBP_Skill_Char OtherActor))
      (Utilities|Array|AddUnique (Variables|Default|GetOverlappedActors) _asbp_skill_char)
      (bind _open (Timeline|OpenDoor PlayFromStart)
        (:Update
          (Transformation|AddWorldOffset (Variables|Default|GetStaticMesh) (Math|Vector|MakeVector 0.0 0.0 _open) false false))
        (:Finished
          (Variables|Default|SetbDoorBusyOpen false)
          (Variables|Default|SetbDoorFinishMove true)
          (Variables|Default|SetbIsOpenned true)
          (Development|PrintString "Door is Open!"))))))

(event OnComponentEndOverlap(TriggerOpen)
  (params (OverlappedComponent :type Primitive%20Component%20Object%20Reference) (OtherActor :type Actor%20Object%20Reference) (OtherComp :type Primitive%20Component%20Object%20Reference) (OtherBodyIndex :type Integer))
  (if (not (and (or (Variables|Default|GetbDoorBusyOpen) (Variables|Default|GetbDoorBusyClose)) (not (Variables|Default|GetbDoorFinishMove))))
    (if (Variables|Default|GetbIsOpenned)
      (Variables|Default|SetbDoorBusyClose true)
      (Variables|Default|SetbDoorFinishMove false)
      (for _array_element (Variables|Default|GetOverlappedActors)
        (if (== _array_element OtherActor)
          (bind _close (Timeline|CloseDoor PlayFromStart)
            (:Update
              (Transformation|AddWorldOffset (Variables|Default|GetStaticMesh) (Math|Vector|MakeVector 0.0 0.0 _close) false false))
            (:Finished
              (Variables|Default|SetbDoorBusyClose false)
              (Variables|Default|SetbDoorFinishMove true)
              (Variables|Default|SetbIsOpenned false)
              (Development|PrintString "Door is Closed!"))))))))

(fn ConstructionScript
  (|CallParentFunction))