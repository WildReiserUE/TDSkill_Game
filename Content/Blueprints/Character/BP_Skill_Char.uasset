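; Player character Blueprint with a zoomable boom camera, aim/walk and sprint speed toggles, and rifle combat.
; A gated, delay-timed fire loop plays montages, spawns projectiles (doubled with DoubleGun), emits AI noise and feeds ammo/reload logic.
; Damage drains armor before health; Death saves state and reopens the Demonstration level.
; BeginPlay creates the HUD and loads the save; F hands possession to Sedan, though SavePlayerParameters is empty.
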(event Custom|LoadGameAfterDead
  ;[1 1 1] LoadGame
  (bind _returnvalue (SaveGame|DoesSaveGameExist "Save"))
  (if _returnvalue
    (bind _returnvalue_2 (SaveGame|LoadGamefromSlot "Save"))
    (bind _asbp_tds_save (Utilities|Casting|CastToBP_SaveGame _returnvalue_2))
    (bind _output_get (Variables|Default|SetSave _asbp_tds_save))
    (Variables|Default|SetXP (Variables|/Game/Blueprints/Interactable/BP_SaveGame.BP_SaveGame_C|GetXP _output_get))
    (Variables|Default|SetUseGun (Variables|/Game/Blueprints/Interactable/BP_SaveGame.BP_SaveGame_C|GetUseGun (Variables|Default|GetSave)))
    ;;[1 1 1] The number of ammo after death is maintained. If you want it to be nullified, just detach the nodes "get ammo" and "get max ammo" from Set Ammo and Set Max Ammo
    (Variables|Default|SetGunAmmo (Variables|/Game/Blueprints/Interactable/BP_SaveGame.BP_SaveGame_C|GetGunAmmo (Variables|Default|GetSave)))
    (Variables|Default|SetGunAmmoMax (Variables|/Game/Blueprints/Interactable/BP_SaveGame.BP_SaveGame_C|GetGunAmmoMax (Variables|Default|GetSave)))
    ;;[1 1 1] Your health and armor after death are restored to their maximum. If you want health and armor to be saved just attach nodes Get Health and get Armor to them
    (Variables|Default|SetHealth 1e+02)
    (Variables|Default|SetArmor 1e+02)
    (if (Variables|Default|GetUseGun)
      (bind _returnvalue_3 (UserInterface|CreateWidget "/Game/Widgets/BP_GunAmmoWidget.BP_GunAmmoWidget_C"))
      (UserInterface|Viewport|AddtoViewport _returnvalue_3 0)
      (Variables|/Game/Blueprints/Interactable/BP_SaveGame.BP_SaveGame_C|SetDead (Variables|Default|GetSave) false)
      (Variables|Default|SetDoubleGun (Variables|/Game/Blueprints/Interactable/BP_SaveGame.BP_SaveGame_C|Get2Guns (Variables|Default|GetSave))))))

(event Custom|LoadBlueGun
  ;[0.08653 0.329 1] LoadGunParameters
  (if (Variables|Default|GetUseGun)
    (Class|SkinnedMeshComponent|SetSkeletalMesh (Variables|Default|GetGun) "/Game/Assets/FirstPerson/FPWeapon/Mesh/SK_FPGunBlue.SK_FPGunBlue" true)
    (bind _returnvalue (UserInterface|CreateWidget "/Game/Widgets/BP_GunAmmoWidget.BP_GunAmmoWidget_C"))
    (UserInterface|Viewport|AddtoViewport _returnvalue 0)))

(event Custom|Car
  (params (Sedan :type BP%20Sedan%20Object%20Reference))
  ;[1 1 1] CarEvent
  (bind _output_get (Variables|Default|SetSedan Sedan))
  (Utilities|IsValid _output_get
    (:Is%20Valid
      (Variables|/Game/Blueprints/Interactable/BP_Sedan.BP_Sedan_C|SetInCar _output_get true))))

(event Custom|LoadPlayerParameters
  ;[1 1 1] LoadPlayerParameters
  (bind _returnvalue (SaveGame|DoesSaveGameExist "Save"))
  (if _returnvalue
    (bind _returnvalue_2 (SaveGame|LoadGamefromSlot "Save"))
    (bind _asbp_tds_save (Utilities|Casting|CastToBP_SaveGame _returnvalue_2))
    (bind _output_get (Variables|Default|SetSave _asbp_tds_save))
    (Variables|Default|SetXP (Variables|/Game/Blueprints/Interactable/BP_SaveGame.BP_SaveGame_C|GetXP _output_get))
    (Variables|Default|SetUseGun (Variables|/Game/Blueprints/Interactable/BP_SaveGame.BP_SaveGame_C|GetUseGun (Variables|Default|GetSave)))
    (Variables|Default|SetGunAmmo (Variables|/Game/Blueprints/Interactable/BP_SaveGame.BP_SaveGame_C|GetGunAmmo (Variables|Default|GetSave)))
    (Variables|Default|SetGunAmmoMax (Variables|/Game/Blueprints/Interactable/BP_SaveGame.BP_SaveGame_C|GetGunAmmoMax (Variables|Default|GetSave)))
    (Variables|Default|SetHealth (Variables|/Game/Blueprints/Interactable/BP_SaveGame.BP_SaveGame_C|GetHealth (Variables|Default|GetSave)))
    (Variables|Default|SetArmor (Variables|/Game/Blueprints/Interactable/BP_SaveGame.BP_SaveGame_C|GetArmor (Variables|Default|GetSave)))
    (Variables|Default|SetDoubleGun (Variables|/Game/Blueprints/Interactable/BP_SaveGame.BP_SaveGame_C|Get2Guns (Variables|Default|GetSave)))
    (if (Variables|Default|GetUseGun)
      (bind _returnvalue_3 (UserInterface|CreateWidget "/Game/Widgets/BP_GunAmmoWidget.BP_GunAmmoWidget_C"))
      (UserInterface|Viewport|AddtoViewport _returnvalue_3 0))))

(event Custom|HUD
  ;[1 1 1] Createw HUD Widget
  (bind _returnvalue (UserInterface|CreateWidget "/Game/Widgets/BP_HUD_Widget.BP_HUD_Widget_C"))
  (UserInterface|Viewport|AddtoViewport _returnvalue 0))

(event Custom|Death
  ;[1 1 1] Death Event
  (if (<= (Variables|Default|GetHealth) 0.0)
    (Utilities|FlowControl|DoOnce false
      (:Completed
        (CallFunction|CameraShakeEvent)
        (Animation|Montage|PlayMontage (Variables|Character|GetMesh) "/Game/Assets/Mannequin/Animations/AnimDeath_1_Montage.AnimDeath_1_Montage"
          (:then
            (Components|DestroyComponent (Variables|Character|GetCharacterMovement))
            (bind _returnvalue (UserInterface|CreateWidget "/Game/Widgets/BP_Death_Widget.BP_Death_Widget_C"))
            (UserInterface|Viewport|AddtoViewport _returnvalue 0)
            (Utilities|FlowControl|Sequence
              (:then_0
                (bind _returnvalue_2 (SaveGame|CreateSaveGameObject "/Game/Blueprints/Interactable/BP_SaveGame.BP_SaveGame_C"))
                (Variables|Default|SetSave _returnvalue_2)
                (Variables|/Game/Blueprints/Interactable/BP_SaveGame.BP_SaveGame_C|SetGunAmmo (Variables|Default|GetSave) (Variables|Default|GetGunAmmo))
                (Variables|/Game/Blueprints/Interactable/BP_SaveGame.BP_SaveGame_C|SetGunAmmoMax (Variables|Default|GetSave) (Variables|Default|GetGunAmmoMax))
                (Variables|/Game/Blueprints/Interactable/BP_SaveGame.BP_SaveGame_C|SetUseGun (Variables|Default|GetSave) (Variables|Default|GetUseGun))
                (Variables|/Game/Blueprints/Interactable/BP_SaveGame.BP_SaveGame_C|SetDead (Variables|Default|GetSave) true)
                (Variables|/Game/Blueprints/Interactable/BP_SaveGame.BP_SaveGame_C|SetXP (Variables|Default|GetSave) (Variables|Default|GetXP))
                (Variables|/Game/Blueprints/Interactable/BP_SaveGame.BP_SaveGame_C|SetInTheCar (Variables|Default|GetSave) (Variables|Default|GetInTheCar))
                (SaveGame|SaveGametoSlot (Variables|Default|GetSave) "Save")
                (Utilities|FlowControl|Delay 2.0)
                (bind _returnvalue_3 (SaveGame|DoesSaveGameExist "Save2"))
                (if _returnvalue_3
                  (bind _returnvalue_4 (SaveGame|LoadGamefromSlot "Save"))
                  (Utilities|Casting|CastToBP_SaveGame _returnvalue_4)
                  (Game|OpenLevel(byName) "Demonstration")
                  (else
                    (Game|OpenLevel(byName) "Demonstration"))))
              (:then_1
                (Utilities|FlowControl|Delay 2.0)
                (Widget|RemovefromParent _returnvalue)))))))))

(event EventBeginPlay
  ;[1 1 1] Begin play
  (CallFunction|HUD)
  (CallFunction|LoadPlayerParameters)
  (CallFunction|Car))

(event Game|Damage|EventAnyDamage
  (params (Damage :type Float%20%28single-precision%29) (DamageType :type Damage%20Type%20Object%20Reference) (InstigatedBy :type Controller%20Object%20Reference) (DamageCauser :type Actor%20Object%20Reference))
  (Variables|Default|SetDamage Damage)
  (if (<= (Variables|Default|GetArmor) 0.0)
    (Variables|Default|SetHealth (- (Variables|Default|GetHealth) (Variables|Default|GetDamage)))
    (else
      (Variables|Default|SetArmor (- (Variables|Default|GetArmor) (Variables|Default|GetDamage))))))

(event Input|MouseEvents|MouseWheelAxis
  (params (AxisValue :type Float%20%28single-precision%29))
  (bind _cameraboom (Variables|Default|GetCameraBoom))
  ;[1 1 1] Camera Zoom In\Out
  (Variables|/Script/Engine.SpringArmComponent|SetTargetArmLength _cameraboom (Math|Float|Clamp(Float) (- (Variables|/Script/Engine.SpringArmComponent|GetTargetArmLength _cameraboom) (* AxisValue (Variables|Camera|GetCameraZoomSpeed))) 3e+02 1.5e+03)))

(event Input|KeyboardEvents|F
  (params (Key :type Key%20Structure :default "None"))
  (bind _returnvalue (Game|GetPlayerController 0))
  (bind _sedan (Variables|Default|GetSedan))
  (:Pressed
    (if (Variables|Default|GetJoinCar)
      (Variables|Default|SetInTheCar true)
      (CallFunction|SavePlayerParameters)
      (Utilities|FlowControl|Delay 0.2)
      (Pawn|UnPossess (Game|GetPlayerController 0))
      (Pawn|Possess (Game|GetPlayerController 0) _sedan)
      (Components|Activation|SetActive (Variables|/Game/Blueprints/Interactable/BP_Sedan.BP_Sedan_C|GetEngineSound _sedan) true false)
      (Actor|DestroyActor)
      (Input|SetInputModeGameOnly _returnvalue)
      (Variables|/Script/Engine.PlayerController|SetbShowMouseCursor _returnvalue false)
      (bind _foundwidgets (Widget|GetAllWidgetsOfClass "/Game/Widgets/BP_HUD_Widget.BP_HUD_Widget_C" false))
      (for _array_element _foundwidgets
        (Widget|RemovefromParent _array_element)
        (bind _foundwidgets_2 (Widget|GetAllWidgetsOfClass "/Game/Widgets/BP_GunAmmoWidget.BP_GunAmmoWidget_C" false))
        (for _array_element_2 _foundwidgets_2
          (Widget|RemovefromParent _array_element_2))))))

(event Input|KeyboardEvents|LeftShift
  (params (Key :type Key%20Structure :default "None"))
  ;[1 1 1] Переключатель Run\Walk\SuperRun\Aiming с проверками
  (:Pressed
    (if (not (Variables|Movement|GetbAimEnabled?))
      (if (Variables|Movement|GetbMoveForward?)
        (CallFunction|RunSuperRunMode)))))

(event Input|MouseEvents|LeftMouseButton
  (params (Key :type Key%20Structure :default "None"))
  (bind _arrow1 (Variables|Default|GetArrow1))
  (bind _mesh (Variables|Character|GetMesh))
  (bind _gunoffset (Variables|Default|GetGunOffset))
  (bind _sphere (Variables|Default|GetSphere))
  (bind _arrow1_2 (Variables|Default|GetArrow1))
  (bind _returnvalue (Transformation|GetWorldRotation _arrow1))
  (bind _returnvalue_2 (Transformation|GetWorldLocation _sphere))
  (bind _returnvalue_3 (Transformation|GetWorldRotation _arrow1_2))
  (bind _returnvalue_4 (Math|Vector|RotateVector _gunoffset _returnvalue_3))
  (bind _returnvalue_5 (+ _returnvalue_2 _returnvalue_4))
  (bind _returnvalue_6 (Math|Transform|MakeTransform _returnvalue_5 _returnvalue_3))
  ;[1 1 1] Anim Fire in Aim and Normal mode
  (:Pressed
    (if (not (Variables|Default|GetReload))
      (if (Variables|Default|GetUseGun)
        (Utilities|FlowControl|Sequence
          (:then_0
            (goto _label Open))
          (:then_1
            (Utilities|FlowControl|Gate true :!label _label
              (:Exit
                (Utilities|FlowControl|Sequence
                  (:then_0
                    (Utilities|FlowControl|RetriggerableDelay 0.2)
                    (goto _label))
                  (:then_1
                    (if (>= (Variables|Default|GetGunAmmo) 1)
                      (if (Variables|Movement|GetbAimEnabled?)
                        (Animation|Montage|PlayMontage _mesh "/Game/Assets/Mannequin/Animations/AnimFire_Rifle_Ironsights_Montage.AnimFire_Rifle_Ironsights_Montage"
                          (:then
                            _))
                        (else
                          (Animation|Montage|PlayMontage _mesh "/Game/Assets/Mannequin/Animations/AnimFire_Rifle_Hip_Montage.AnimFire_Rifle_Hip_Montage"
                            (:then
                              _))))
                      (Variables|Default|SetGunAmmo (- (Variables|Default|GetGunAmmo) 1))
                      (Game|SpawnActorfromClass "/Game/Blueprints/Interactable/BP_CharacterProjectile.BP_CharacterProjectile_C" (Math|Transform|MakeTransform (Math|Vector|MakeVector (.x (.location _returnvalue_6)) (.y (.location _returnvalue_6)) (.z (Transformation|GetActorLocation))) (.rotation _returnvalue_6) (.scale _returnvalue_6)) "AlwaysSpawn" 0 0) ; Spawn projectile
                      (Audio|PlaySoundatLocation "/Game/FX_A/Audio/Wav/ShootSound_Wav.ShootSound_Wav" (Transformation|GetActorLocation) "0, 0, 0" 1.0 1.0 0.0 0 0 0) ; Play firing sound
                      (Class|PawnNoiseEmitterComponent|MakeNoise (Variables|Default|GetPawnNoiseEmitter) self 1.0 (Transformation|GetActorLocation))
                      ;[1 1 1] When you find a double gun, another projectile is added.
                      (if (Variables|Default|GetDoubleGun)
                        (Game|SpawnActorfromClass "/Game/Blueprints/Interactable/BP_CharacterProjectile.BP_CharacterProjectile_C" (Math|Transform|MakeTransform (+ (Transformation|GetWorldLocation (Variables|Default|GetArrow1)) (Math|Vector|RotateVector (Variables|Default|GetGunOffset) _returnvalue)) _returnvalue) "AdjustIfPossibleButDontSpawnIfColliding" 0 0) ; Spawn projectile
                      ))))))))))))

(event Input|MouseEvents|LeftMouseButton
  (params (Key :type Key%20Structure :default "None"))
  (bind _arrow1 (Variables|Default|GetArrow1))
  (bind _mesh (Variables|Character|GetMesh))
  (bind _gunoffset (Variables|Default|GetGunOffset))
  (bind _sphere (Variables|Default|GetSphere))
  (bind _arrow1_2 (Variables|Default|GetArrow1))
  (bind _returnvalue (Transformation|GetWorldRotation _arrow1))
  (bind _returnvalue_2 (Transformation|GetWorldLocation _sphere))
  (bind _returnvalue_3 (Transformation|GetWorldRotation _arrow1_2))
  (bind _returnvalue_4 (Math|Vector|RotateVector _gunoffset _returnvalue_3))
  (bind _returnvalue_5 (+ _returnvalue_2 _returnvalue_4))
  (bind _returnvalue_6 (Math|Transform|MakeTransform _returnvalue_5 _returnvalue_3))
  ;[1 1 1] Anim Fire in Aim and Normal mode
  (:Released
    (Utilities|FlowControl|Gate true) ; enters at Close
  ))

(event Input|MouseEvents|RightMouseButton
  (params (Key :type Key%20Structure :default "None"))
  ;[1 1 1] Переключатель Run\Walk\SuperRun\Aiming с проверками
  (:Pressed
    (Variables|Movement|SetbAimEnabled? true)
    (if (Variables|Movement|GetbCharacterFastRun)
      (CallFunction|RunSuperRunMode))
    (CallFunction|RunWalkMode :!label _label))
  (:Released
    (Variables|Movement|SetbAimEnabled? false)
    (goto _label)))

(event Input|KeyboardEvents|R
  (params (Key :type Key%20Structure :default "None"))
  (:Pressed
    (if (Variables|Default|GetUseGun)
      (if (>= (Variables|Default|GetGunAmmoMax) 1)
        (Variables|Default|SetNeedAmmo (- 30 (Variables|Default|GetGunAmmo)))
        (if (<= (Variables|Default|GetGunAmmoMax) (Variables|Default|GetNeedAmmo))
          (Variables|Default|SetGunAmmo (+ (Variables|Default|GetGunAmmo) (Variables|Default|GetGunAmmoMax)))
          (Variables|Default|SetGunAmmoMax 0)
          (else
            (Variables|Default|SetGunAmmoMax (- (Variables|Default|GetGunAmmoMax) (Variables|Default|GetNeedAmmo)))
            (Variables|Default|SetGunAmmo 30)))
        (Variables|Default|SetReload true)
        (Audio|Components|Audio|Play (Variables|Default|GetReloadSound1) 0.0)
        (Animation|Montage|PlayMontage (Variables|Character|GetMesh) "/Game/Assets/Mannequin/Animations/AnimReload_Rifle_Hip_Montage.AnimReload_Rifle_Hip_Montage"
          (:then
            (bind _foundwidgets (Widget|GetAllWidgetsOfClass "/Game/Widgets/BP_GunAmmoWidget.BP_GunAmmoWidget_C" false))
            (for _array_element _foundwidgets
              (Class|UserWidget|PlayAnimationForward _array_element (Variables|/Game/Widgets/BP_GunAmmoWidget.BP_GunAmmoWidget_C|GetButtonAnim _array_element) 1.0 false)
              (Class|UserWidget|PlayAnimationForward _array_element (Variables|/Game/Widgets/BP_GunAmmoWidget.BP_GunAmmoWidget_C|GetTextAnim _array_element) 1.0 false)
              (Class|UserWidget|PlayAnimationForward _array_element (Variables|/Game/Widgets/BP_GunAmmoWidget.BP_GunAmmoWidget_C|GetTextAnimation _array_element) 1.0 false)
              (Utilities|FlowControl|Delay 1.0)))
          (:OnCompleted
            (Variables|Default|SetReload false)))))))

(fn ConstructionScript
  (bind _cameraboom (Variables|Default|GetCameraBoom))
  (Variables|/Script/Engine.SpringArmComponent|SetTargetArmLength _cameraboom (Variables|Camera|GetCameraLenght))
  (Transformation|SetRelativeRotation _cameraboom (Variables|Camera|GetCameraRotation) false false)
  (Variables|/Script/Engine.SpringArmComponent|SetbEnableCameraLag _cameraboom (Variables|Camera|GetCameraLag))
  (Variables|/Script/Engine.SpringArmComponent|SetCameraLagSpeed _cameraboom (Variables|Camera|GetCameraLagDelay))
  (Variables|Movement|SetbCharacterWalk (Variables|Movement|GetbCharacterWalk)))

(fn CameraShakeEvent
  (Camera|PlayWorldCameraShake "/Game/Blueprints/Effects/BP_CameraMatenee.BP_CameraMatenee_C" (Transformation|GetWorldLocation (Variables|Default|GetTopDownCameraComponent)) 0.0 2e+01))

(fn RunWalkMode
  (bind _coefslowwalk (Variables|Movement|GetCoefSlowWalk))
  (bind _charactermovement (Variables|Character|GetCharacterMovement))
  (if (Variables|Movement|GetbAimEnabled?)
    (Development|PrintString "Aim" true true "(R=1.000000,G=0.300000,B=0.000000,A=1.000000)" 5.0)
    (Variables|/Script/Engine.CharacterMovementComponent|SetMaxWalkSpeed _charactermovement (/ (Variables|/Script/Engine.CharacterMovementComponent|GetMaxWalkSpeed _charactermovement) _coefslowwalk))
    (Variables|Movement|SetbCharacterWalk true)
    (else
      (Development|PrintString "Run" true true "(R=0.000000,G=1.000000,B=0.000000,A=1.000000)" 5.0)
      (Variables|/Script/Engine.CharacterMovementComponent|SetMaxWalkSpeed _charactermovement (* (Variables|/Script/Engine.CharacterMovementComponent|GetMaxWalkSpeed _charactermovement) _coefslowwalk))
      (Variables|Movement|SetbCharacterWalk false))))

(fn RunSuperRunMode
  (bind _coeffastrun (Variables|Movement|GetCoefFastRun))
  (bind _charactermovement (Variables|Character|GetCharacterMovement))
  ;[1 1 1] проверяем текущий режим ходьбы или бега
  (if (not (Variables|Movement|GetbCharacterWalk))
    ;[1 1 1] Уже бежим?
    (if (Variables|Movement|GetbCharacterFastRun)
      ;;[1 1 1] сбрасываем скорость если уже бежим и бежим если не  бежали
      (Variables|/Script/Engine.CharacterMovementComponent|SetMaxWalkSpeed _charactermovement (/ (Variables|/Script/Engine.CharacterMovementComponent|GetMaxWalkSpeed _charactermovement) _coeffastrun))
      (Development|PrintString "NormalRun" true true "(R=1.000000,G=0.300000,B=0.000000,A=1.000000)" 5.0)
      (Variables|Movement|SetbCharacterFastRun false)
      (else
        (Variables|/Script/Engine.CharacterMovementComponent|SetMaxWalkSpeed _charactermovement (* (Variables|/Script/Engine.CharacterMovementComponent|GetMaxWalkSpeed _charactermovement) _coeffastrun))
        (Development|PrintString "FastRun" true true "(R=0.000000,G=1.000000,B=0.000000,A=1.000000)" 5.0)
        (Variables|Movement|SetbCharacterFastRun true)))))

(fn SavePlayerParameters)