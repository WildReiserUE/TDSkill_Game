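; Ammo pickup for the blue gun that raises the player character's GunAmmoMax when touched.
; Box overlap casts to BP_Skill_Char and applies the increase before checking CanExecuteCosmeticEvents.
; Only when that check passes does it play the pickup cue, remove the box, text and rune, show BP_Ammo_Widget, and destroy the actor after a short delay.
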(event OnComponentBeginOverlap(Box)
  (params (OverlappedComponent :type Primitive%20Component%20Object%20Reference) (OtherActor :type Actor%20Object%20Reference) (OtherComp :type Primitive%20Component%20Object%20Reference) (OtherBodyIndex :type Integer) (bFromSweep :type Boolean) (SweepResult :type Hit%20Result%20Structure%20%28by%20ref%29))
  ;[1 1 1] Pick Up Ammo for Blue Gun
  (bind _asbp_skill_char (Utilities|Casting|CastToBP_Skill_Char OtherActor))
  (Variables|/Game/Blueprints/Character/BP_Skill_Char.BP_Skill_Char_C|SetGunAmmoMax _asbp_skill_char (+ (Variables|/Game/Blueprints/Character/BP_Skill_Char.BP_Skill_Char_C|GetGunAmmoMax _asbp_skill_char) 100))
  (Networking|CanExecuteCosmeticEvents
    (:True
      (Audio|Components|Audio|Play (Variables|Default|GetPickUp_Cue) 0.0)
      (Components|DestroyComponent (Variables|Default|GetBox))
      (bind _returnvalue (UserInterface|CreateWidget "/Game/Widgets/BP_+Ammo_Widget.BP_+Ammo_Widget_C"))
      (UserInterface|Viewport|AddtoViewport _returnvalue 0)
      (Components|DestroyComponent (Variables|Default|GetRune_P2))
      (Utilities|FlowControl|Delay 1.0)
      (Actor|DestroyActor))))

(fn ConstructionScript)